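; Test enemy AI that uses pawn sensing to chase and attack a seen pawn, with checks for PC and VR players.
; Each sighting triggers a server event that moves to the pawn, then sends a damage message gated by CanAttack and a delay.
; Health is cached only for PC players and decremented locally; the VR branch only checks the cast.
; The attack montage node is disconnected from execution, and Tick does nothing.
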(event OnSeePawn(PawnSensing)
  (params (Pawn :type Pawn%20Object%20Reference))
  (Variables|Default|SetIs_Seeing_Player? true)
  (CallFunction|SERVER:FollowPLayer)
  (if (Actor|ActorHasTag Pawn "PC-Player")
    (bind _asbp_first_person_character (Utilities|Casting|CastToBP_FirstPersonCharacter Pawn)
      (:then
        (Variables|Default|SetHealth_Player (Variables|/Game/Managment/FirstPerson/Blueprints/BP_FirstPersonCharacter.BP_FirstPersonCharacter_C|GetHealth _asbp_first_person_character)))
      (:CastFailed
        (Development|PrintText "pc player cast fallido")))
    (elif (Actor|ActorHasTag Pawn "VR-Player")
      (Utilities|Casting|CastToVRPawn Pawn
        (:CastFailed
          (Development|PrintText "casteo vr pawn fallido"))))))

(event Custom|SERVER:Follow_PLayer
  (if (Variables|Default|GetIs_Seeing_Player?)
    (Variables|Default|SetCan_Attack? true)
    (AI|AIMoveTo self "0, 0, 0" (stale OnSeePawn(PawnSensing) Pawn) 7e+01 false
      (:OnSuccess
        (if (Variables|Default|GetCan_Attack?)
          (Variables|Default|SetCan_Attack? false)
          (Class|BPINPCAttackPlayer|NpcAttack-ToPlayer(Message) (stale OnSeePawn(PawnSensing) Pawn) (Variables|Default|GetDamage) (Variables|Default|GetName_NPC))
          (Variables|Default|SetHealth_Player (- (Variables|Default|GetHealth_Player) (Variables|Default|GetDamage)))
          (Utilities|FlowControl|Delay (stale _returnvalue))
          (Variables|Default|SetCan_Attack? true))))
    (else
      (Variables|Default|SetIs_Seeing_Player? false))))

(event EventBeginPlay)

(event Collision|EventActorBeginOverlap
  (params (OtherActor :type Actor%20Object%20Reference)))

(event EventTick
  (params (DeltaSeconds :type Float%20%28single-precision%29))
  (if (Variables|Default|GetIs_Seeing_Player?)
    _))

(fn ConstructionScript)