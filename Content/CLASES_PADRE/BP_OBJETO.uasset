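; BP_OBJETO is a base item Blueprint, apparently for pickups that go into the VR pawn's inventory component.
; Its overlap and interact events are empty, and the PickupItem function only returns false.
; Disconnected logic would add OBJETO and its CANTIDAD to ACINVENTARIOEQUIPMENT and destroy the actor, in one variant only when the other actor is tagged MENU, but none of it runs.
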(event Collision|EventActorBeginOverlap
  (params (OtherActor :type Actor%20Object%20Reference)))

(event EventMENSAJEINTERACTUAR
  (params (OVERLAP :type Boolean) (HELD_REALEASED :type Boolean)))

(fn ConstructionScript)

(fn Pickup-Item
  (params (ID :type Name :default "None") (Drop_Item :type S%20Inventory%20Item%20Structure))
  (return false))