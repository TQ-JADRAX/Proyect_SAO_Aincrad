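; Test pickup item actor whose appearance and item data come from a DAPickUp data asset.
; The construction script sets the static mesh from that asset.
; Logic to add the item's name, description, icon, quantity, weight and damage to the ACINVENTARIOEQUIPMENT inventory and then destroy the actor is present but disconnected.
; The MENSAJEINTERACTUAR interaction event is empty, so interacting currently does nothing.
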(event EventBeginPlay)

(event Collision|EventActorBeginOverlap
  (params (OtherActor :type Actor%20Object%20Reference)))

(event EventTick
  (params (DeltaSeconds :type Float%20%28single-precision%29)))

(event EventMENSAJEINTERACTUAR
  (params (OVERLAP :type Boolean) (HELD_REALEASED :type Boolean)))

(fn ConstructionScript
  (Components|StaticMesh|SetStaticMesh (Variables|Default|GetStaticMesh) (Variables|/Game/DATA_ASSET/BP_Pickup.BP_Pickup_C|GetStatic_Mesh (Variables|Default|GetDA_PickUp))))