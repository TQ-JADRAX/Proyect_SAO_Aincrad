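; Inventory component for the SAO menu item system, storing items in a map of slot structs keyed by item name.
; GetItem reports whether a slot's quantity is above zero, and AddItem increases that quantity or creates a new slot with zeroed values.
; DropItem subtracts from the quantity inside the nested item struct, not the slot quantity, and removes the entry at zero or below.
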(event EventBeginPlay)

(event EventTick
  (params (DeltaSeconds :type Float%20%28single-precision%29)))

(fn GetItem
  (params (Item :type S%20Item%20Structure))
  (bind _s_slot (Variables|Default|GetS_slot))
  (bind (_value _returnvalue) (Utilities|Map|Find _s_slot (.name_item Item)))
  (if _returnvalue
    (return (> (.Cantidad (Utilities|Struct|BreakS_Slot_Inventory_Item _value)) 0))
    (else
      (return false))))

(fn AddItem
  (params (Item :type S%20Item%20Structure) (Cantidad :type Integer))
  (bind _name_item (Utilities|Struct|BreakS_Item Item))
  (bind _s_slot (Variables|Default|GetS_slot))
  (bind (_value _returnvalue) (Utilities|Map|Find _s_slot _name_item))
  (if _returnvalue
    (bind _structout (Utilities|Struct|SetmembersinS_Slot_Inventory_Item _value (+ (.Cantidad (Utilities|Struct|BreakS_Slot_Inventory_Item _value)) Cantidad)))
    (Utilities|Map|Add (Variables|Default|GetS_slot) (.name_item Item) _structout)
    (else
      (Utilities|Map|Add _s_slot _name_item (Utilities|Struct|MakeS_Slot_Inventory_Item Item 0 0))))
  (return))

(fn DropItem
  (params (Item :type S%20Item%20Structure) (Cantidad :type Integer))
  (bind _s_slot (Variables|Default|GetS_slot))
  (bind (_value _returnvalue) (Utilities|Map|Find _s_slot (.name_item Item)))
  (bind _item (Utilities|Struct|BreakS_Slot_Inventory_Item _value))
  (bind _returnvalue_2 (- (.cantidad _item) Cantidad))
  (if _returnvalue
    (if (<= _returnvalue_2 0)
      (Utilities|Map|Remove (Variables|Default|GetS_slot) (.name_item Item))
      (else
        (bind _structout (Utilities|Struct|SetmembersinS_Slot_Inventory_Item _value (Utilities|Struct|MakeS_Item (.name_item _item) (.descripcion _item) (.actor _item) (.static_mesh _item) (.icono _item) _returnvalue_2 (.cantidad_maxima _item) (.durabilidad _item) (.armadura _item) (.? _item))))
        (Utilities|Map|Add (Variables|Default|GetS_slot) (.name_item Item) _structout)))))