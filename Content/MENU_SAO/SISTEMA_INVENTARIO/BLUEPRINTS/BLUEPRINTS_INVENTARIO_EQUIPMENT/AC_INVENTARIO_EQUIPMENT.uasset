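; Actor component that holds the equipment inventory in a VR game as a SLOT map of item and quantity, keyed by item name.
; ADD stacks quantity or creates an entry once the player pawn casts to VRPawn, then calls CARGARSLOTS on REF to reload slots.
; DROP subtracts quantity and removes emptied entries without that reload.
; GET reports whether an item exists and whether its count strictly exceeds the requested amount.
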(event EventBeginPlay)

(event EventTick
  (params (DeltaSeconds :type Float%20%28single-precision%29)))

(fn ADD
  (params (OBJETO :type S%20OBJETO%20Structure) (CANTIDAD :type Integer))
  (bind _name (Utilities|Struct|BreakS_OBJETO OBJETO))
  (bind _slot (Variables|Default|GetSLOT))
  (bind (_value _returnvalue) (Utilities|Map|Find _slot _name))
  (Utilities|Casting|CastToVRPawn (Game|Player|GetPlayerPawn 0))
  (if _returnvalue
    (bind _structout (Utilities|Struct|SetmembersinS_INVENTORY_SLOT _value (+ (.CANTIDAD (Utilities|Struct|BreakS_INVENTORY_SLOT _value)) CANTIDAD)))
    (Utilities|Map|Add (Variables|Default|GetSLOT) (.name OBJETO) _structout)
    (else
      (Utilities|Map|Add (Variables|Default|GetSLOT) _name (Utilities|Struct|MakeS_INVENTORY_SLOT OBJETO CANTIDAD))))
  (Default|CARGARSLOTS (Variables|Default|GetREF))
  (return false))

(fn DROP
  (params (OBJETO :type S%20OBJETO%20Structure) (CANTIDAD :type Integer))
  (bind _slot (Variables|Default|GetSLOT))
  (bind (_value _returnvalue) (Utilities|Map|Find _slot (.name OBJETO)))
  (bind _cantidad (Utilities|Struct|BreakS_INVENTORY_SLOT _value))
  (bind _returnvalue_2 (- _cantidad CANTIDAD))
  (if _returnvalue
    (if (<= _returnvalue_2 0)
      (Utilities|Map|Remove (Variables|Default|GetSLOT) (.name OBJETO))
      (else
        (bind _structout (Utilities|Struct|SetmembersinS_INVENTORY_SLOT _value _returnvalue_2))
        (Utilities|Map|Add (Variables|Default|GetSLOT) (.name OBJETO) _structout)))))

(fn GET
  (params (OBJETO :type S%20OBJETO%20Structure) (CANTIDAD :type Integer))
  (bind _slot (Variables|Default|GetSLOT))
  (bind (_value _returnvalue) (Utilities|Map|Find _slot (.name OBJETO)))
  (if _returnvalue
    (return true (> (.CANTIDAD (Utilities|Struct|BreakS_INVENTORY_SLOT _value)) CANTIDAD))
    (else
      (return false false))))