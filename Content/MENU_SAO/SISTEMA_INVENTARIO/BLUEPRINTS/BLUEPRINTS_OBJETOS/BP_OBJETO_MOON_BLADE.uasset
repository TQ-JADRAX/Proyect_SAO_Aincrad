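; Pickup actor for the Moon Blade item in the inventory system, which adds itself to the player's equipment inventory.
; Overlap with an actor tagged MENU adds the item and its quantity to the VRPawn's ACINVENTARIOEQUIPMENT, then destroys the pickup; other overlaps print a debug string.
; The MENSAJEINTERACTUAR interaction event does the same through the passed player reference, without the tag check.
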(event EventBeginPlay
  (|CallParentFunction))

(event Collision|EventActorBeginOverlap
  (params (OtherActor :type Actor%20Object%20Reference))
  (if (Actor|ActorHasTag OtherActor "MENU")
    (Default|ADD (Variables|/Game/VRTemplate/Blueprints/VRPawn.VRPawn_C|GetAC_INVENTARIO_EQUIPMENT (.AsVRPawn (Utilities|Casting|CastToVRPawn (Game|Player|GetPlayerPawn 0)))) (Variables|Default|GetOBJETO) (.cantidad (Variables|Default|GetDETAILS)))
    (Actor|DestroyActor)
    (else
      (Development|PrintString "OVERLAP_FALSE"))))

(event EventTick
  (params (DeltaSeconds :type Float%20%28single-precision%29))
  (|CallParentFunction DeltaSeconds) ; Este nodo está deshabilitado y no se le llamará.\nArrastra pines para construir una funcionalidad.
)

(event EventMENSAJEINTERACTUAR
  (params (REFERENCIA_JUGADOR :type VR%20Pawn%20Object%20Reference))
  (Default|ADD (Variables|/Game/VRTemplate/Blueprints/VRPawn.VRPawn_C|GetAC_INVENTARIO_EQUIPMENT REFERENCIA_JUGADOR) (Variables|Default|GetOBJETO) (.cantidad (Variables|Default|GetDETAILS)))
  (Actor|DestroyActor))

(fn ConstructionScript
  (|CallParentFunction))