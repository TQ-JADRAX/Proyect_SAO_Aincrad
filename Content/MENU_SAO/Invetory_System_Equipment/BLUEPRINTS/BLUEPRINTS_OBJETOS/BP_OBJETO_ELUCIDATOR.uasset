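; BP_OBJETO_ELUCIDATOR is the pickup actor for the Elucidator item in the SAO menu's inventory and equipment system.
; Its MENSAJEINTERACTUAR event, when OVERLAP is true, adds OBJETO with the quantity from DETAILS to the player VRPawn's ACINVENTARIOEQUIPMENT component, then destroys the actor.
; A false OVERLAP only prints a debug string.
; Tick and overlap events do nothing, and an older add-and-destroy chain is left unconnected.
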(event EventBeginPlay
  (|CallParentFunction))

(event Collision|EventActorBeginOverlap
  (params (OtherActor :type Actor%20Object%20Reference)))

(event EventTick
  (params (DeltaSeconds :type Float%20%28single-precision%29))
  (|CallParentFunction DeltaSeconds) ; Este nodo está deshabilitado y no se le llamará.\nArrastra pines para construir una funcionalidad.
)

(event EventMENSAJEINTERACTUAR
  (params (OVERLAP :type Boolean) (HELD_REALEASED :type Boolean))
  (if OVERLAP
    (Default|ADD (Variables|/Game/VRTemplate/Blueprints/VRPawn.VRPawn_C|GetAC_INVENTARIO_EQUIPMENT (.AsVRPawn (Utilities|Casting|CastToVRPawn (Game|Player|GetPlayerPawn 0)))) (Variables|Default|GetOBJETO) (.cantidad (Variables|Default|GetDETAILS)))
    (Actor|DestroyActor)
    (else
      (Development|PrintString "OVERLAP_FALSE"))))

(fn ConstructionScript
  (|CallParentFunction))