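; World pickup actor that displays an inventory item and shows a name prompt to the nearby local player.
; OnRep_ID, also run on construction and BeginPlay, looks up ID in DT_Inventory, preferring DropItem data when set.
; Update sets the prompt text, then blocking-loads either the holdable Blueprint as a child actor or, failing that, a static mesh.
; Sphere overlaps toggle the widget for locally controlled non-AI players, and Tick turns it toward the camera.
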(event OnComponentBeginOverlap(Sphere)
  (params (OverlappedComponent :type Primitive%20Component%20Object%20Reference) (OtherActor :type Actor%20Object%20Reference) (OtherComp :type Primitive%20Component%20Object%20Reference) (OtherBodyIndex :type Integer) (bFromSweep :type Boolean) (SweepResult :type Hit%20Result%20Structure%20%28by%20ref%29))
  ;[0.15 0.15 0.15 0.5] Change_Visibility_(Widget_Interact)
  (bind _asbp_first_person_character (Utilities|Casting|CastToBP_FirstPersonCharacter OtherActor))
  (if (Actor|ActorHasTag OtherActor "BP_First-Person(player)")
    (Utilities|IsPLayer(PC) _asbp_first_person_character
      (:verdadero
        (Rendering|SetVisibility (Variables|Default|GetWidget) true false)
        (Variables|Default|SetPlayer_%28PC%29_is_Overlaping? true)))))

(event OnComponentEndOverlap(Sphere)
  (params (OverlappedComponent :type Primitive%20Component%20Object%20Reference) (OtherActor :type Actor%20Object%20Reference) (OtherComp :type Primitive%20Component%20Object%20Reference) (OtherBodyIndex :type Integer))
  ;[0.15 0.15 0.15 0.5] Change_Visibility_(Widget_Interact)
  (bind _asbp_first_person_character (Utilities|Casting|CastToBP_FirstPersonCharacter OtherActor))
  (if (Actor|ActorHasTag OtherActor "BP_First-Person(player)")
    (Utilities|IsPLayer(PC) _asbp_first_person_character
      (:verdadero
        (Rendering|SetVisibility (Variables|Default|GetWidget) false false)
        (Variables|Default|SetPlayer_%28PC%29_is_Overlaping? false)))))

(event Custom|Update
  (bind _item (Variables|Default|GetItem))
  (bind _staticmesh (Variables|Default|GetStaticMesh))
  (bind (_display_name _static_mesh _skeletal_mesh _holdable_settings) (Utilities|Struct|BreakS_Inventory_Item _item))
  (bind _aswbp_pickup__item (Utilities|Casting|CastToWBP_Pickup-Item (UserInterface|GetWidget (Variables|Default|GetWidget))))
  (Rendering|Components|TextRender|SetText (Variables|/Game/System_Inventorys/Widgets_PC_Pickup/WBP_Pickup-Item.WBP_Pickup-Item_C|GetText_Interact _aswbp_pickup__item) _display_name)
  (bind _returnvalue (Utilities|LoadClassAssetBlocking (.bp_actor _holdable_settings)))
  (bind _asactor (Utilities|Casting|CastToActorClass _returnvalue)
    (:then
      (ChildActorComponent|SetChildActorClass (Variables|Default|GetChildActor) _asactor))
    (:CastFailed
      (bind _returnvalue_2 (Utilities|LoadAssetBlocking _static_mesh))
      (bind _asstatic_mesh (Utilities|Casting|CastToStaticMesh _returnvalue_2))
      (Components|StaticMesh|SetStaticMesh _staticmesh _asstatic_mesh)
      (Collision|SetCollisionEnabled _staticmesh "QueryAndPhysics")
      (Collision|SetCollisionObjectType _staticmesh "ECC_WorldStatic"))))

(event EventBeginPlay
  (CallFunction|OnRepID)
  (Collision|SetCollisionEnabled (Variables|Default|GetStaticMesh) "NoCollision"))

(event Collision|EventActorBeginOverlap
  (params (OtherActor :type Actor%20Object%20Reference)))

(event EventTick
  (params (DeltaSeconds :type Float%20%28single-precision%29))
  (Utilities|FlowControl|Sequence
    (:then_0
      (if (Variables|Default|GetPlayer_%28PC%29_is_Overlaping?)
        (Utilities|Casting|CastToBP_FirstPersonCharacter (Game|Player|GetPlayerPawn 0))
        ;[0.03434 0.03434 0.03434] Rotate Widget towards camera
        (Transformation|SetWorldRotation (Variables|Default|GetWidget) (Math|Rotator|FindLookatRotation (Transformation|GetWorldLocation (Variables|Default|GetWidget)) (Camera|GetCameraLocation (Game|GetPlayerCameraManager 0))) false false)))))

(fn ConstructionScript
  (CallFunction|OnRepID))

(fn OnRepID
  (bind _returnvalue (Utilities|GetDataTableRow "/Game/System_Inventorys/Data_Tables_Inventory/DT_Inventory.DT_Inventory" (Variables|Default|GetID))
    (:then
      (Variables|Default|SetItem (select (!= (Utilities|Struct|BreakS_Inventory_Item (Variables|Default|GetDrop_Item)) "") (Variables|Default|GetDrop_Item) _returnvalue))
      (CallFunction|Update))))