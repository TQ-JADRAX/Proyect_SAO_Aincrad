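; Player controller that picks and spawns the player's pawn at startup, either for VR or for flat-screen play.
; On BeginPlay it checks whether HMD data is valid, then spawns a VR pawn or a BP_FirstPersonCharacter at the first PlayerStart found and possesses it.
; The VR pawn spawns lowered on Z from the PlayerStart, while the first-person character uses its transform unchanged.
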(event EventBeginPlay
  (bind _hmddata (Class|HeadMountedDisplayFunctionLibrary|GetHMDData))
  (if (.bValid (Utilities|Struct|BreakXRHMDData _hmddata))
    (bind _returnvalue (Actor|GetActorOfClass "/Script/Engine.PlayerStart"))
    (bind _returnvalue_2 (Game|SpawnActorfromClass "/Game/VRTemplate/Blueprints/VRPawn.VRPawn_C" (Math|Transform|MakeTransform (Math|Vector|MakeVector (.X (Math|Vector|BreakVector (.location (Transformation|GetActorTransform _returnvalue)))) (.Y (Math|Vector|BreakVector (.location (Transformation|GetActorTransform _returnvalue)))) (- (.Z (Math|Vector|BreakVector (.location (Transformation|GetActorTransform _returnvalue)))) 92.0)) (.rotation (Transformation|GetActorTransform _returnvalue)) (.scale (Transformation|GetActorTransform _returnvalue))) "AlwaysSpawn" "MultiplyWithRoot" 0 0))
    (Pawn|Possess _returnvalue_2)
    (else
      (bind _returnvalue_3 (Actor|GetActorOfClass "/Script/Engine.PlayerStart"))
      (bind _returnvalue_4 (Game|SpawnActorfromClass "/Game/FirstPerson/Blueprints/BP_FirstPersonCharacter.BP_FirstPersonCharacter_C" (Transformation|GetActorTransform _returnvalue_3) "AlwaysSpawn" "MultiplyWithRoot" 0 0))
      (Pawn|Possess _returnvalue_4))))

(fn ConstructionScript)